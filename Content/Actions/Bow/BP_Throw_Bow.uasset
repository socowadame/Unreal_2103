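; Bow projectile actor that damages what its Sphere overlaps, ignoring its owner and actors of the owner's class.
; On a valid overlap it applies Data.Power damage, credited to the controller of the owning Character.
; It then spawns the optional Data.Effect emitter at the target, offset and scaled by Data.EffectTransform and yawed along the projectile-to-target direction, and destroys itself.
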(event OnComponentBeginOverlap(Sphere)
  (params (OverlappedComponent :type Primitive%20Component%20Object%20Reference) (OtherActor :type Actor%20Object%20Reference) (OtherComp :type Primitive%20Component%20Object%20Reference) (OtherBodyIndex :type Integer) (bFromSweep :type Boolean) (SweepResult :type Hit%20Result%20Structure%20%28by%20ref%29))
  (bind _self self)
  (bind _data (Variables|Default|GetData))
  (bind (_location _rotation _scale) (Math|Transform|BreakTransform (.effecttransform _data)))
  (Utilities|FlowControl|Sequence
    (:then_0
      (if (and (!= OtherActor (Components|GetOwner)) (!= (Utilities|GetClass OtherActor) (Utilities|GetClass (Components|GetOwner))))
        (bind _ascharacter (Utilities|Casting|CastToCharacter (Components|GetOwner)))
        (Game|Damage|ApplyDamage OtherActor (.power _data) (Pawn|GetController _ascharacter) _self)
        (Utilities|FlowControl|Sequence
          (:then_0
            (Utilities|IsValid (.effect _data)
              (:Is%20Valid
                (Effects|SpawnEmitteratLocation (.effect _data) (+ (Transformation|GetActorLocation OtherActor) _location) (Math|Rotator|MakeRotator 0.0 0.0 (.yaw (Math|Rotator|FindLookatRotation (Transformation|GetActorLocation _self) (Transformation|GetActorLocation OtherActor)))) _scale))))
          (:then_1
            (Actor|DestroyActor)))))))

(fn ConstructionScript
  (|CallParentFunction))