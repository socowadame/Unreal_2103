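; Equipment Blueprint that handles equipping and unequipping an attachment for its owning character, tracking the equipped flag.
; Equip sets the equip state, plays the data-driven montage or completes immediately without one, then applies movement permission, controller-yaw rotation and character color.
; Begin and end events notify the attachment and restore idle and movement through the owner's State and Status components.
; Unequip notifies the attachment and restores orient-to-movement rotation.
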(event Custom|Begin_Equip
  (Default|OnEquip (Variables|Default|GetAttachment)))

(event Custom|End_Equip
  (Default|SetIdleMode (Variables|Default|GetState))
  (Default|SetMove (Variables|Default|GetStatus))
  (Variables|Default|SetEquipped true))

(event Custom|Equip
  (bind _data (Variables|Default|GetData))
  (bind _status (Variables|Default|GetStatus))
  (Default|SetEquipMode (Variables|Default|GetState))
  (Utilities|FlowControl|Sequence
    (:then_0
      (if (Utilities|IsValid (.animmontage _data))
        (bind _ascharacter (Utilities|Casting|CastToCharacter (Components|GetOwner)))
        (Animation|PlayAnimMontage _ascharacter (.animmontage _data) (.playratio _data) (.startsection _data))
        (else
          (CallFunction|BeginEquip)
          (CallFunction|EndEquip))))
    (:then_1
      (if (.canmove _data)
        (Default|SetMove _status)
        (else
          (Default|SetStop _status))))
    (:then_2
      (if (.pawncontrol _data)
        (bind _ascharacter_2 (Utilities|Casting|CastToCharacter (Components|GetOwner)))
        (Variables|/Script/Engine.Pawn|SetbUseControllerRotationYaw _ascharacter_2 true)
        (Variables|/Script/Engine.CharacterMovementComponent|SetbOrientRotationToMovement (Variables|/Script/Engine.Character|GetCharacterMovement _ascharacter_2) false)))
    (:then_3
      (bind _asicharacter (Utilities|Casting|CastToICharacter (Components|GetOwner)))
      (Default|ChangeColor _asicharacter (.color (Variables|Default|GetData))))))

(event Custom|Unequip
  (Default|OnUnequip (Variables|Default|GetAttachment))
  (bind _ascharacter (Utilities|Casting|CastToCharacter (Components|GetOwner)))
  (Variables|/Script/Engine.Pawn|SetbUseControllerRotationYaw _ascharacter false)
  (Variables|/Script/Engine.CharacterMovementComponent|SetbOrientRotationToMovement (Variables|/Script/Engine.Character|GetCharacterMovement _ascharacter) true)
  (Variables|Default|SetEquipped false))

(event EventBeginPlay
  (Variables|Default|SetState (Actor|GetComponentbyClass (Components|GetOwner) "/Game/Components/StateComponent.StateComponent_C"))
  (Variables|Default|SetAction (Actor|GetComponentbyClass (Components|GetOwner) "/Game/Components/ActionComponent.ActionComponent_C"))
  (Variables|Default|SetStatus (Actor|GetComponentbyClass (Components|GetOwner) "/Game/Components/StatusComponent.StatusComponent_C")))

(fn ConstructionScript)

(fn GetEquipped
  (return (Variables|Default|GetEquipped)))