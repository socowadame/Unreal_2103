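; BP_Attachment_Fist is the fist attachment actor, which mounts its sphere components onto the owning character's skeletal mesh.
; On BeginPlay it runs the parent logic, then attaches each sphere to the mesh socket matching that component's object name, keeping relative transforms.
; Each sphere has collision disabled once attached, and the loop requires the owner to be a Character.
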(event EventBeginPlay
  (|CallParentFunction)
  (for _array_element (Actor|GetComponentsByClass "/Script/Engine.SphereComponent")
    (bind _ascharacter (Utilities|Casting|CastToCharacter (Components|GetOwner)))
    (Transformation|AttachComponentToComponent _array_element (Variables|/Script/Engine.Character|GetMesh _ascharacter) (Utilities|String|StringToName (Utilities|GetObjectName _array_element)) "KeepRelative" "KeepRelative" "KeepRelative" true)
    (Collision|SetCollisionEnabled _array_element "NoCollision")))

(fn ConstructionScript
  (|CallParentFunction))