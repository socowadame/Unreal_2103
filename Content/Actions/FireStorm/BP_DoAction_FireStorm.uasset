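; FireStorm combat action that sends an attachment's box component circling its owner, repeatedly damaging characters it overlaps.
; DoAction switches from idle to action mode and plays the action, whose begin step shows the box and enables collision.
; Tick orbits the box by rotating an offset around Z, while overlaps maintain a hit list damaged by a looping timer.
; The end step starts a delay timer, and OnFinish hides the box and restores idle.
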(event EventTick
  (params (DeltaSeconds :type Float%20%28single-precision%29))
  (if (Math|Boolean|ANDBoolean (CallFunction|GetEquipped) (Default|IsActionMode (Variables|Default|GetState)) (Utilities|IsValid (CallFunction|GetBox)))
    (Utilities|FlowControl|Sequence
      (:then_0
        (bind _output_get (Variables|Default|SetAngle (+ (* DeltaSeconds (Variables|Default|GetSpeed)) (Variables|Default|GetAngle))))
        (if (Math|Float|NearlyEqual(Float) _output_get 3.6e+02 1e-06)
          (Variables|Default|SetAngle 0.0)))
      (:then_1
        (Utilities|IsValid (CallFunction|GetBox)
          (:Is%20Valid
            (Transformation|SetWorldLocation (CallFunction|GetBox) (- (+ (Math|Vector|RotateVectorAroundAxis (Math|Vector|MakeVector (Variables|Default|GetDistance) 0.0 0.0) (Variables|Default|GetAngle) "0, 0,1.000000") (Transformation|GetActorLocation (Variables|Default|GetOwnerCharacter))) (Math|Vector|MakeVector 0.0 0.0 (Variables|Default|GetHeight))) false false)))))))

(fn ConstructionScript
  (|CallParentFunction))

(fn DoAction
  (bind _state (Variables|Default|GetState))
  (|CallParentFunction)
  (if (Default|IsIdleMode _state)
    (Default|SetActionMode _state)
    (CallFunction|PlayAction)))

(fn BeginDoAction
  (bind _outputpin (CallFunction|GetBox))
  (|CallParentFunction)
  (Utilities|IsValid _outputpin
    (:Is%20Valid
      (Rendering|SetVisibility _outputpin true true)
      (Utilities|Time|SetTimerbyFunctionName self "OnHitted" 0.1 true)
      (Collision|SetCollisionEnabled (CallFunction|GetBox) "QueryAndPhysics"))))

(fn EndDoAction
  (|CallParentFunction)
  (Utilities|Time|SetTimerbyEvent (EventDispatchers|CreateEvent :!event OnFinish) (Variables|Default|GetTimer)))

(fn GetBox
  (bind _ownercharacter (Variables|Default|GetOwnerCharacter))
  (bind _returnvalue (Actor|GetComponentbyClass _ownercharacter "/Game/Components/ActionComponent.ActionComponent_C"))
  (bind _attachment (Default|GetAttachment _returnvalue))
  (bind _returnvalue_2 (Actor|GetComponentbyClass _attachment "/Script/Engine.BoxComponent"))
  (Utilities|IsValid _returnvalue
    (:Is%20Valid
      (Utilities|IsValid _returnvalue_2
        (:Is%20Valid
          (return _returnvalue_2))))))

(fn OnFinish
  (Rendering|SetVisibility (CallFunction|GetBox) false true)
  (Utilities|Time|ClearTimerbyFunctionName self "OnHitted")
  (Collision|SetCollisionEnabled (CallFunction|GetBox) "NoCollision")
  (Default|SetIdleMode (Variables|Default|GetState)))

(fn OnAttachmentBeginOverlap
  (params (OtherCharacter :type Character%20Object%20Reference))
  (|CallParentFunction 0)
  (Utilities|Array|AddUnique (Variables|Default|GetHittedCharacters) OtherCharacter))

(fn OnAttachmentEndOverlap
  (params (OtherCharacter :type Character%20Object%20Reference))
  (|CallParentFunction 0)
  (Utilities|Array|RemoveItem (Variables|Default|GetHittedCharacters) OtherCharacter))

(fn OnHitted
  (for _array_element (Variables|Default|GetHittedCharacters)
    (CallFunction|SendDamage _array_element)))