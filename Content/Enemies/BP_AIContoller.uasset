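; AI controller for BP_AI enemies that runs the pawn's behavior tree and tracks a visible player.
; On possession, it starts the BehaviorTree assigned on the BP_AI pawn, printing a failure message if none is valid.
; Every tick, it polls AIPerception's sight sense for a BP_Player, updating or clearing the "Player" blackboard object key.
; The detected player's name is printed for debugging.
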(event Custom|UpdatedBreak
  (Utilities|Array|ForEachLoopwithBreak (Class|AIPerceptionComponent|GetCurrentlyPerceivedActors (Variables|Default|GetAIPerception) "/Script/AIModule.AISense_Sight")) ; enters at Break
)

(event EventTick
  (params (DeltaSeconds :type Float%20%28single-precision%29))
  (Variables|Default|SetFindPlayer false)
  (bind _array_element (Utilities|Array|ForEachLoopwithBreak (Class|AIPerceptionComponent|GetCurrentlyPerceivedActors (Variables|Default|GetAIPerception) "/Script/AIModule.AISense_Sight"))
    (:LoopBody
      (bind _asbp_player (Utilities|Casting|CastToBP_Player _array_element))
      (AI|Components|Blackboard|SetValueasObject (AI|GetBlackboard 0) (Utilities|Name|MakeLiteralName "Player") _asbp_player)
      (Variables|Default|SetFindPlayer true)
      (CallFunction|UpdatedBreak))
    (:Completed
      (if (Variables|Default|GetFindPlayer)
        (Development|PrintString (Utilities|GetDisplayName _asbp_player) true true "(R=0.000000,G=0.660000,B=1.000000,A=1.000000)" 0.0)
        (else
          (AI|Components|Blackboard|SetValueasObject (AI|GetBlackboard 0) (Utilities|Name|MakeLiteralName "Player") 0))))))

(event EventPossess
  (params (PossessedPawn :type Pawn%20Object%20Reference))
  (bind _asbp_ai (Utilities|Casting|CastToBP_AI PossessedPawn))
  (Utilities|IsValid (Variables|/Game/Enemies/BP_AI.BP_AI_C|GetBehaviorTree _asbp_ai)
    (:Is%20Valid
      (AI|RunBehaviorTree (Variables|/Game/Enemies/BP_AI.BP_AI_C|GetBehaviorTree _asbp_ai)))
    (:Is%20Not%20Valid
      (Development|PrintString "Fail"))))

(fn ConstructionScript)