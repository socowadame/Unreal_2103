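; Enemy character that takes player damage, reacts to hits and drops a BP_ITems pickup on death.
; SetDamage scales damage by player stats with a random critical, updates the combo UI and lowers StatusComponent health.
; Surviving hits play a reaction montage, rotate via LookAtAttacker, flash dynamic materials red and knock back from melee.
; Death sets dead state, plays its montage, then destroys the actor and spawns the item after a delay.
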(event EventBeginPlay
  (Utilities|FlowControl|Sequence
    (:then_0
      (bind _returnvalue (Rendering|Material|CreateDynamicMaterialInstance "/Game/Materials/M_UE4Man_Body_Inst.M_UE4Man_Body_Inst" "None" :!class /Script/Engine.KismetMaterialLibrary))
      (Utilities|Array|Add (Variables|Default|GetMaterials) _returnvalue)
      (bind _returnvalue_2 (Rendering|Material|CreateDynamicMaterialInstance "/Game/Materials/M_UE4Man_ChestLogo_Inst.M_UE4Man_ChestLogo_Inst" "None" :!class /Script/Engine.KismetMaterialLibrary))
      (Utilities|Array|Add (Variables|Default|GetMaterials) _returnvalue_2)
      (Rendering|Material|SetMaterial (Variables|Character|GetMesh) 0 (Utilities|Array|Get(acopy) (Variables|Default|GetMaterials)))
      (Rendering|Material|SetMaterial (Variables|Character|GetMesh) 1 (Utilities|Array|Get(acopy) (Variables|Default|GetMaterials) 1)))
    (:then_1
      (bind _aswb_label (Utilities|Casting|CastToWB_Label (UserInterface|GetUserWidgetObject (Variables|Default|GetLabel))))
      (Default|UpdateCharacter _aswb_label (Math|Conversions|ToInteger(Byte) (Utilities|String|Replace (Utilities|GetObjectName self) "BP_Enemy"))))))

(event Game|Damage|EventAnyDamage
  (params (Damage :type Float%20%28single-precision%29) (DamageType :type Damage%20Type%20Object%20Reference) (InstigatedBy :type Controller%20Object%20Reference) (DamageCauser :type Actor%20Object%20Reference))
  (bind _returnvalue (Transformation|GetActorTransform))
  (bind _statecomponent (Variables|Default|GetStateComponent))
  (bind (_x _y _z) (Math|Vector|BreakVector (.location _returnvalue)))
  (|SetDamage DamageCauser InstigatedBy Damage
    (:then
      (Default|SetHittedMode _statecomponent)
      (Animation|PlayAnimMontage "/Game/Character/Montages/Common/Enemy_HitReaction_Montage.Enemy_HitReaction_Montage" 1.5 "None")
      (|LookAtAttacker)
      (for _array_element (Variables|Default|GetMaterials)
        (|ChangeColor _array_element)
        (|Launch (Variables|Default|GetCauser))))
    (:Dead
      (if (not (Default|IsDeadMode _statecomponent))
        (Default|SetDeadMode (Variables|Default|GetStateComponent))
        (Default|PlayDead (Variables|Default|GetMontagesComponent))
        (Utilities|FlowControl|Delay 3.0)
        (Actor|DestroyActor self)
        (Game|SpawnActorfromClass "/Game/Items/BP_ITems.BP_ITems_C" (Math|Transform|MakeTransform (Math|Vector|MakeVector _x _y (- _z 92.0)) (.rotation _returnvalue) (.scale _returnvalue)) "AlwaysSpawn" 0 0)))))

(fn ConstructionScript)

(fn ChangeColor
  (params (InColor :type Linear%20Color%20Structure))
  (return false))

(fn EndBackstep
  (return false))

(fn EndDead
  (Actor|DestroyActor)
  (return false))

(fn EndHurri
  (return false))

(fn EndRoll
  (return false))

(event EventTick
  (params (DeltaSeconds :type Float%20%28single-precision%29)))