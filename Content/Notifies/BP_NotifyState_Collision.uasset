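; Animation notify state, displayed as "Collision", that switches collision on and off for an attachment during a window of an animation.
; On begin, it looks up the attachment from the animated skeletal mesh through NotifyGetAttachment and, if valid, calls OnCollision.
; On end, it repeats the same lookup and calls OffCollision, leaving the collision behavior itself to the attachment.
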(fn GetNotifyName
  (return "Collision"))

(fn ReceivedNotifyBegin
  (params (MeshComp :type Skeletal%20Mesh%20Component%20Object%20Reference) (Animation :type Anim%20Sequence%20Base%20Object%20Reference) (TotalDuration :type Float%20%28single-precision%29))
  (bind _attachment (CallFunction|NotifyGetAttachment MeshComp MeshComp))
  (Utilities|IsValid _attachment
    (:Is%20Valid
      (Default|OnCollision _attachment)
      (return false))))

(fn ReceivedNotifyEnd
  (params (MeshComp :type Skeletal%20Mesh%20Component%20Object%20Reference) (Animation :type Anim%20Sequence%20Base%20Object%20Reference))
  (bind _attachment (CallFunction|NotifyGetAttachment MeshComp MeshComp))
  (Utilities|IsValid _attachment
    (:Is%20Valid
      (Default|OffCollision _attachment)
      (return false))))