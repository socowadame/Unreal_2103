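; Animation notify state named "Combo" that marks the combo window inside melee attack animations.
; On begin and end it looks up the current DoAction from the mesh and casts it to BP_DoAction_Melee.
; It calls OnCombo when the window opens and OffCombo when it closes, doing nothing if the action is missing or not melee.
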(fn GetNotifyName
  (return "Combo"))

(fn ReceivedNotifyBegin
  (params (MeshComp :type Skeletal%20Mesh%20Component%20Object%20Reference) (Animation :type Anim%20Sequence%20Base%20Object%20Reference) (TotalDuration :type Float%20%28single-precision%29))
  (bind _do_action (CallFunction|NotifyGetDoAction MeshComp MeshComp))
  (Utilities|IsValid _do_action
    (:Is%20Valid
      (bind _asbp_do_action_melee (Utilities|Casting|CastToBP_DoAction_Melee _do_action))
      (Default|OnCombo _asbp_do_action_melee)
      (return false))))

(fn ReceivedNotifyEnd
  (params (MeshComp :type Skeletal%20Mesh%20Component%20Object%20Reference) (Animation :type Anim%20Sequence%20Base%20Object%20Reference))
  (bind _do_action (CallFunction|NotifyGetDoAction MeshComp MeshComp))
  (Utilities|IsValid _do_action
    (:Is%20Valid
      (bind _asbp_do_action_melee (Utilities|Casting|CastToBP_DoAction_Melee _do_action))
      (Default|OffCombo _asbp_do_action_melee)
      (return false))))