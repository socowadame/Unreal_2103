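; BP_ITems is a pickup actor that randomly becomes one of two item types on BeginPlay, showing the matching aura component.
; When the player overlaps its sphere, it calls either Updatedamage or Updatemagic on BP_Player, then destroys itself.
; The player's Angry state raises the amount passed to Updatedamage, while Updatemagic always receives a fixed amount.
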(event OnComponentBeginOverlap(Sphere)
  (params (OverlappedComponent :type Primitive%20Component%20Object%20Reference) (OtherActor :type Actor%20Object%20Reference) (OtherComp :type Primitive%20Component%20Object%20Reference) (OtherBodyIndex :type Integer) (bFromSweep :type Boolean) (SweepResult :type Hit%20Result%20Structure%20%28by%20ref%29))
  (bind _returnvalue (Game|GetPlayerCharacter 0))
  (bind _asbp_player (Utilities|Casting|CastToBP_Player _returnvalue))
  (if (== OtherActor _returnvalue)
    (if (Variables|/Game/Player/BP_Player.BP_Player_C|GetAngry _asbp_player)
      (Variables|Default|Setitemeffect 15.0)
      (else
        (Variables|Default|Setitemeffect 3.0)))
    (switch int (stale EventBeginPlay _output_get)
      (:0
        (Default|Updatedamage _asbp_player (Variables|Default|Getitemeffect)))
      (:1
        (Default|Updatemagic _asbp_player 3.0)))
    (Actor|DestroyActor)))

(event EventBeginPlay
  (bind _output_get (Variables|Default|Setset (Math|Random|RandomInteger 2)))
  (switch int _output_get
    (:0
      (Rendering|SetVisibility (Variables|Default|GetP_ky_auroraAura) true false))
    (:1
      (Rendering|SetVisibility (Variables|Default|GetP_ky_auroraAura1) true false))))

(event Collision|EventActorBeginOverlap
  (params (OtherActor :type Actor%20Object%20Reference)))

(event EventTick
  (params (DeltaSeconds :type Float%20%28single-precision%29)))

(fn ConstructionScript)