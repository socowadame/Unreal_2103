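; BP_11_Dot is a debug demo that visualizes the dot product between a Player's facing and the direction to an Enemy.
; Each tick it draws a blue arrow from the Player to its scaled forward vector, not offset by its location, and a red arrow to the Enemy.
; It also prints the dot product of the Player's forward vector and the normalized direction to the Enemy.
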(event EventTick
  (params (DeltaSeconds :type Float%20%28single-precision%29))
  (Utilities|FlowControl|Sequence
    (:then_0
      (Rendering|Debug|DrawDebugArrow (Transformation|GetActorLocation (Variables|Default|GetPlayer)) (* (Transformation|GetActorForwardVector (Variables|Default|GetPlayer)) 1e+03) 1e+02 "(R=0.000000,G=0.000000,B=1.000000,A=1.000000)" 0.0 0.0))
    (:then_1
      (Rendering|Debug|DrawDebugArrow (Transformation|GetActorLocation (Variables|Default|GetPlayer)) (Transformation|GetActorLocation (Variables|Default|GetEnemy)) 1e+02 "(R=1.000000,G=0.000000,B=0.000000,A=1.000000)" 0.0 0.0))
    (:then_2
      (Development|PrintString (Utilities|String|ToString(Float) (Math|Vector|DotProduct (Transformation|GetActorForwardVector (Variables|Default|GetPlayer)) (Math|Vector|Normalize (- (Transformation|GetActorLocation (Variables|Default|GetEnemy)) (Transformation|GetActorLocation (Variables|Default|GetPlayer))))))))))

(fn ConstructionScript)