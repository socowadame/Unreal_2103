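; BP_11_Cross is a debug demo that visualizes the vector cross product between a Player and an Enemy.
; Each Tick draws arrows from the Player toward scaled forward, Enemy location, and forward × to-Enemy cross product.
; The forward and cross vectors serve directly as world-space end points, without adding Player location.
; It prints Enemy location, the cross vector, and its dot with Player up, a signed left/right indicator.
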(event EventTick
  (params (DeltaSeconds :type Float%20%28single-precision%29))
  (bind _player (Variables|Default|GetPlayer))
  (bind _player_2 (Variables|Default|GetPlayer))
  (bind _enemy (Variables|Default|GetEnemy))
  (bind _returnvalue (Transformation|GetActorForwardVector _player))
  (bind _returnvalue_2 (Transformation|GetActorLocation _player_2))
  (bind _returnvalue_3 (Transformation|GetActorLocation _enemy))
  (bind _returnvalue_4 (- _returnvalue_3 _returnvalue_2))
  (bind _returnvalue_5 (Math|Vector|CrossProduct _returnvalue _returnvalue_4))
  (Utilities|FlowControl|Sequence
    (:then_0
      (Rendering|Debug|DrawDebugArrow (Transformation|GetActorLocation (Variables|Default|GetPlayer)) (* (Transformation|GetActorForwardVector (Variables|Default|GetPlayer)) 1e+03) 1e+02 "(R=0.000000,G=0.000000,B=1.000000,A=1.000000)" 0.0 0.0))
    (:then_1
      (Rendering|Debug|DrawDebugArrow (Transformation|GetActorLocation (Variables|Default|GetPlayer)) (Transformation|GetActorLocation (Variables|Default|GetEnemy)) 1e+02 "(R=1.000000,G=0.000000,B=0.000000,A=1.000000)" 0.0 0.0))
    (:then_2
      (Rendering|Debug|DrawDebugArrow (Transformation|GetActorLocation (Variables|Default|GetPlayer)) _returnvalue_5 1e+02 "(R=0.000000,G=1.000000,B=0.000000,A=1.000000)" 0.0 0.0)
      (Development|PrintString (Utilities|String|Append (Utilities|String|ToString(Vector) (Transformation|GetActorLocation (Variables|Default|GetEnemy))) " / " (Utilities|String|ToString(Vector) _returnvalue_5) " / " (Utilities|String|ToString(Float) (Math|Vector|DotProduct _returnvalue_5 (Transformation|GetActorUpVector (Variables|Default|GetPlayer)))))))))

(fn ConstructionScript)